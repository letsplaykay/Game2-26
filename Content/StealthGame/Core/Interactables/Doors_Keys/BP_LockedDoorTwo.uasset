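; BP_LockedDoorTwo is an interactable locked door that opens when the player character holds more than one key.
; Overlapping its box collision casts to BP_ThirdPersonCharacter and checks KeyCount, then plays a timeline that lerps the door mesh's yaw to swing it open.
; Without enough keys it prints a locked-door message to the screen.
; Key removal and the door-open sound are present but disconnected, so keys are not consumed.
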(event `self.Box collision.OnComponentBeginOverlap`
  (params (OverlappedComponent :type "PrimitiveComponent Object Reference") (OtherActor :type "Actor Object Reference") (OtherComp :type "PrimitiveComponent Object Reference") (OtherBodyIndex :type Integer) (bFromSweep :type Boolean) (SweepResult :type "HitResult Structure (by ref)"))
  (bind _asbp_third_person_character (cast `/Game/ThirdPerson/Blueprints/BP_ThirdPersonCharacter` OtherActor))
  (if (> (`/Game/ThirdPerson/Blueprints/BP_ThirdPersonCharacter.Key Count` _asbp_third_person_character) 1)
    (bind (_direction _rotationrate) (`Timeline|Timeline`)
      (:`Update`
        (`SceneComponent.K2_SetRelativeRotation` (`self.SM_Door`) (`KismetMathLibrary.MakeRotator` 0.0 0.0 (`KismetMathLibrary.Lerp` 0.0 -90.0 _rotationrate)) false false)))
    (else
      (`KismetSystemLibrary.PrintString` "Get More Keys! Door is locked" true true (struct :`R` 0.479167 :`G` 0.051103 :`A` 1.0) 5.0))))

(fn `UserConstructionScript`)